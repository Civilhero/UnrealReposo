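; BP_TimelineDoor is a door actor that rises when the third-person character overlaps it, then lowers itself.
; Overlap sets an open flag and plays the OpenDoor timeline, while Tick watches that flag, waits through a short Delay, clears it and plays DoorClose.
; Both timelines serve only as update tickers, adding a fixed unswept vertical offset per update, so travel distance depends on frame rate.
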(event EventBeginPlay)

(event Collision|EventActorBeginOverlap
  (params (OtherActor :type Actor%20Object%20Reference))
  (if (not (Variables|Default|GetIsDoorOpen))
    (Utilities|Casting|CastToBP_ThirdPersonCharacter OtherActor)
    (Variables|Default|SetIsDoorOpen true)
    (Timeline|Open%20Door Play
      (:Update
        (Transformation|AddActorWorldOffset "0.000000,0.000000,50.000000")))))

(event EventTick
  (params (DeltaSeconds :type Float%20%28single-precision%29))
  (if (Variables|Default|GetIsDoorOpen)
    (Utilities|FlowControl|Delay 2.0)
    (Variables|Default|SetIsDoorOpen false)
    (Timeline|DoorClose Play
      (:Update
        (Transformation|AddActorWorldOffset "0.000000,0.000000,-50.000000")))))

(fn ConstructionScript)